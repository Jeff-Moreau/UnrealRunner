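; BP_PickupJump is a pickup actor that grants the player a jump ability when touched.
; On overlap with the player character, it sets BP_Player's jump Z velocity to a fixed value.
; It then records the pickup in the GlobalGameInstance flag GIsPickupJump and destroys itself.
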(event `self.ReceiveActorBeginOverlap`
  (params (OtherActor :type "Actor Object Reference"))
  (bind _returnvalue (`GameplayStatics.GetPlayerCharacter` 0))
  (if (== OtherActor _returnvalue)
    (bind _asbp_player (cast `/Game/Blueprints/Player/BP_Player` _returnvalue))
    (set `CharacterMovementComponent.JumpZVelocity` 600.0 (`Character.CharacterMovement` _asbp_player))
    (bind _asglobal_game_instance (cast `/Game/GlobalGameInstance` (`GameplayStatics.GetGameInstance`)))
    (bind _output_get (set `self.Globals` _asglobal_game_instance))
    (set `/Game/GlobalGameInstance.GIsPickupJump` true _output_get)
    (`self.K2_DestroyActor`)))

(fn `UserConstructionScript`)