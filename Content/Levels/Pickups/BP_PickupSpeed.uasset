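; Speed pickup actor that boosts the player's walk speed when collected.
; On overlap with player character 0, it sets the BP_Player movement component's max walk speed to a fixed value and plays a 2D sound.
; It then sets the GIsPickupSpeed flag on the GlobalGameInstance and destroys itself.
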(event `self.ReceiveActorBeginOverlap`
  (params (OtherActor :type "Actor Object Reference"))
  (bind _returnvalue (`GameplayStatics.GetPlayerCharacter` 0))
  (if (== OtherActor _returnvalue)
    (bind _asbp_player (cast `/Game/Blueprints/Player/BP_Player` _returnvalue))
    (set `CharacterMovementComponent.MaxWalkSpeed` 500.0 (`Character.CharacterMovement` _asbp_player))
    (`GameplayStatics.PlaySound2D` "/Game/Audio/effect_notify-84408.effect_notify-84408" 1.0 1.0 0.0 null null)
    (bind _asglobal_game_instance (cast `/Game/GlobalGameInstance` (`GameplayStatics.GetGameInstance`)))
    (bind _output_get (set `self.Globals` _asglobal_game_instance))
    (set `/Game/GlobalGameInstance.GIsPickupSpeed` true _output_get)
    (`self.K2_DestroyActor`)))

(fn `UserConstructionScript`)