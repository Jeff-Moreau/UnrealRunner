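; Fog pickup that temporarily changes the killer fog speed stored in the GlobalGameInstance when the player touches it.
; BeginPlay caches the game instance and resets the fog speed to its default.
; On player overlap it raises that value, plays a 2D sound and makes its sprite transparent.
; After a short delay it restores the default and destroys itself.
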(event `self.ReceiveBeginPlay`
  (bind _asglobal_game_instance (cast `/Game/GlobalGameInstance` (`GameplayStatics.GetGameInstance`)))
  (set `self.Globals` _asglobal_game_instance)
  (set `/Game/GlobalGameInstance.GKillerFogSpeed` 3.0 (`self.Globals`)))

(event `self.ReceiveActorBeginOverlap`
  (params (OtherActor :type "Actor Object Reference"))
  (if (== OtherActor (`GameplayStatics.GetPlayerCharacter` 0))
    (set `/Game/GlobalGameInstance.GKillerFogSpeed` 5.0 (`self.Globals`))
    (`GameplayStatics.PlaySound2D` "/Game/Audio/dark-and-frightening-click-142377.dark-and-frightening-click-142377" 1.0 1.0 0.0 null null)
    (`PaperSpriteComponent.SetSpriteColor` :`self` (`self.PaperSprite`))
    (`KismetSystemLibrary.Delay` 3.0)
    (set `/Game/GlobalGameInstance.GKillerFogSpeed` 3.0 (`self.Globals`))
    (`self.K2_DestroyActor`)))

(fn `UserConstructionScript`)