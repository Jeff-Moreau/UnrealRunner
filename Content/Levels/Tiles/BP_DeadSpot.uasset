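; BP_DeadSpot is a level tile hazard that marks the player as hit when the player touches it.
; Both actor overlap and blocking hit events check for player character 0 and cast it to BP_Player.
; Either path then sets IsHit and switches PlayerCurrentState to a fixed enum value, leaving any further response outside this Blueprint.
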(event `self.ReceiveActorBeginOverlap`
  (params (OtherActor :type "Actor Object Reference"))
  (bind _returnvalue (`GameplayStatics.GetPlayerCharacter` 0))
  (if (== OtherActor _returnvalue)
    (bind _asbp_player (cast `/Game/Blueprints/Player/BP_Player` _returnvalue))
    (set `/Game/Blueprints/Player/BP_Player.IsHit` true _asbp_player)
    (set `/Game/Blueprints/Player/BP_Player.PlayerCurrentState` "NewEnumerator2" _asbp_player)))

(event `self.ReceiveHit`
  (params (MyComp :type "PrimitiveComponent Object Reference") (Other :type "Actor Object Reference") (OtherComp :type "PrimitiveComponent Object Reference") (bSelfMoved :type Boolean) (HitLocation :type "Vector Structure") (HitNormal :type "Vector Structure") (NormalImpulse :type "Vector Structure") (Hit :type "HitResult Structure (by ref)"))
  (bind _returnvalue (`GameplayStatics.GetPlayerCharacter` 0))
  (if (== Other _returnvalue)
    (bind _asbp_player (cast `/Game/Blueprints/Player/BP_Player` _returnvalue))
    (set `/Game/Blueprints/Player/BP_Player.IsHit` true _asbp_player)
    (set `/Game/Blueprints/Player/BP_Player.PlayerCurrentState` "NewEnumerator2" _asbp_player)))

(fn `UserConstructionScript`)